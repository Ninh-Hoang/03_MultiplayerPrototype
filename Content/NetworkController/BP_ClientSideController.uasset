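; Player controller for networked click-to-move play, splitting each player into a client-side camera pawn and a server-side character.
; After BeginPlay, the server moves the pawn to a random PlayerStart, then spawns the character and a server-side controller that possesses it.
; Tick captures the cursor's world hit and repositions the pawn by interpolation with the character's location.
; Left click has the server controller move the character there, beyond a minimum distance.
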(event `Server_init Player`
  ;[1 1 1] Server Init Player
  (bind _asbp_client_side_pawn (cast `/Game/NetworkController/BP_ClientSidePawn` (`self.K2_GetPawn`)))
  (bind _output_get (set `self.ClientSidePawnRef` _asbp_client_side_pawn))
  (set `ClientSidePawn.ClientSideControllerRef` self _output_get)
  (`self.Server Spawn Player`))

(event `self.ReceiveBeginPlay`
  ;[1 1 1] Client Side Init Player
  (`KismetSystemLibrary.Delay` 0.5)
  (set `self.bShowMouseCursor` true)
  (`self.Server_init Player`))

(event `Server Spawn Player`
  (bind _clientsidepawnref (`self.ClientSidePawnRef`))
  (bind _returnvalue (`self.GetTransform` _clientsidepawnref))
  ;[1 1 1] Server Side Spawning
  (`/Engine/EditorBlueprintResources/ActorMacros.Switch Has Authority`
    (:`Authority`
      (bind _outactors (`GameplayStatics.GetAllActorsOfClass` "/Script/Engine.PlayerStart"))
      (`/Engine/EditorBlueprintResources/StandardMacros.DoOnce` false
        (:`Completed`
          (`self.K2_SetActorLocation` _clientsidepawnref (`self.K2_GetActorLocation` (`|GetArrayItem` _outactors (`KismetMathLibrary.RandomIntegerInRange` 0 (`KismetArrayLibrary.Array_LastIndex` _outactors)))) false true)
          (bind _returnvalue_2 (`|SpawnActorFromClass` "/Game/NetworkController/BP_ServerSideCharacter.BP_ServerSideCharacter_C" _returnvalue "AdjustIfPossibleButAlwaysSpawn" "OverrideRootScale" null null))
          (set `self.ServerSideCharacterRef` _returnvalue_2)
          (bind _asnetwork_player_state (cast `NetworkPlayerState` (`self.PlayerState`)))
          (set `NetworkPlayerState.ServerSideCharacterRef` (`self.ServerSideCharacterRef`) _asnetwork_player_state)
          (bind _returnvalue_3 (`|SpawnActorFromClass` "/Game/NetworkController/BP_ServerSideController.BP_ServerSideController_C" _returnvalue "Undefined" "OverrideRootScale" null self null))
          (bind _output_get (set `self.ServerSideControllerRef` _returnvalue_3))
          (set `ServerSideController.ServerSideCharacterRef` (`self.ServerSideCharacterRef`) _output_get)
          (`self.Possess` (`self.ServerSideControllerRef`) (`self.ServerSideCharacterRef`)))))))

(event `Server Move Server Character`
  (params (`Mouse Location` :type "Vector Structure"))
  (bind _serversidecontrollerref (`self.ServerSideControllerRef`))
  ;[1 1 1] Server move server character to mouse location
  (`/Engine/EditorBlueprintResources/ActorMacros.Switch Has Authority`
    (:`Authority`
      (if (>= (`KismetMathLibrary.VSize` (- (`self.K2_GetActorLocation` (`self.ServerSideCharacterRef`)) `Mouse Location`)) (`self.MinimumClickDistance`))
        (`/Engine/EditorBlueprintResources/StandardMacros.IsValid` _serversidecontrollerref
          (:`Is Valid`
            (`AIController.MoveToLocation` _serversidecontrollerref `Mouse Location` -1.0 true true false true null true)))))))

(event `Client Mouse Capture`
  (bind (_bblockinghit _binitialoverlap _time _distance _location) (`GameplayStatics.BreakHitResult` (`self.GetHitResultUnderCursorByChannel` "TraceTypeQuery1")))
  ;[1 1 1] Client Mouse Location Capture
  (if _bblockinghit
    (set `self.MouseLocation` _location)))

(event `Client Update Camera`
  (params (DeltaTime :type "Float (double-precision)"))
  (bind _serversidecharacterref (`self.ServerSideCharacterRef`))
  ;[1 1 1] Client Camera Update
  (`/Engine/EditorBlueprintResources/StandardMacros.IsValid` _serversidecharacterref
    (:`Is Valid`
      (`self.K2_SetActorLocation` (`self.ClientSidePawnRef`) (`KismetMathLibrary.VInterpTo` (`self.K2_GetActorLocation` _serversidecharacterref) (`self.K2_GetActorLocation` (`self.ClientSidePawnRef`)) DeltaTime 10.0) false false))))

(event `Key|LeftMouseButton`
  (params (Key :type "Key Structure"))
  ;[1 1 1] Have Server Controller Move Server Character To Mouse Location
  (:`Pressed`
    (`/Engine/EditorBlueprintResources/StandardMacros.IsValid` (`self.ServerSideControllerRef`)
      (:`Is Valid`
        (`self.Server Move Server Character` (`self.MouseLocation`))))))

(event `self.ReceiveTick`
  (params (DeltaSeconds :type "Float (single-precision)"))
  ;[1 1 1] Delta Time Tick
  (`|ExecutionSequence`
    (:`then_0`
      (`self.Client Mouse Capture`))
    (:`then_1`
      (`self.Client Update Camera` DeltaSeconds))))

(fn `UserConstructionScript`)